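; FollowCam is a Blueprint actor with a FollowCam component that turns to face the first player while a FollowArea trigger switches it on and off.
; Any begin overlap on FollowArea activates the component and any end overlap deactivates it, with no actor filtering.
; Tick sets its world rotation every frame via FindLookAtRotation toward the player controller's actor location rather than the pawn's, regardless of active state.
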(event OnComponentBeginOverlap(FollowArea)
  (params (OtherActor :type Actor%20Object%20Reference) (OtherComp :type Primitive%20Component%20Object%20Reference) (OtherBodyIndex :type Integer) (bFromSweep :type Boolean) (SweepResult :type Hit%20Result%20Structure%20%28by%20ref%29))
  (Components|Activation|SetActive (Variables|Default|GetFollowCam) true false))

(event OnComponentEndOverlap(FollowArea)
  (params (OtherActor :type Actor%20Object%20Reference) (OtherComp :type Primitive%20Component%20Object%20Reference) (OtherBodyIndex :type Integer))
  (Components|Activation|SetActive (Variables|Default|GetFollowCam) false false))

(event EventTick
  (params (DeltaSeconds :type Float%20%28single-precision%29))
  (bind _followcam (Variables|Default|GetFollowCam))
  (Transformation|SetWorldRotation _followcam (Math|Rotator|FindLookatRotation (Transformation|GetWorldLocation _followcam) (Transformation|GetActorLocation (Game|GetPlayerController 0))) false false))

(fn ConstructionScript)