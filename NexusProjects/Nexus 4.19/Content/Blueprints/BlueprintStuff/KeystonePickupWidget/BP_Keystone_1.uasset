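; BP_Keystone_1 is a pickup actor for the first keystone, collected when the ThirdPersonCharacter overlaps its Box.
; On overlap it sends the Keystone1 inventory message, adds a keystone to the character, plays a sound, spawns an explosion effect and destroys itself.
; It sets Collected1 on the Nexus_GameInstance and checks that flag on BeginPlay, removing itself if already collected so the pickup stays gone across level loads.
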(event OnComponentBeginOverlap(Box)
  (params (OtherActor :type Actor%20Object%20Reference) (OtherComp :type Primitive%20Component%20Object%20Reference) (OtherBodyIndex :type Integer) (bFromSweep :type Boolean) (SweepResult :type Hit%20Result%20Structure%20%28by%20ref%29))
  (bind _asnexus_game_instance (Utilities|Casting|CastToNexus_GameInstance (Game|GetGameInstance)))
  (bind _asthird_person_character (Utilities|Casting|CastToThirdPersonCharacter OtherActor))
  (Class|InventoryInterface|AddInventory(Message) OtherActor (Variables|/Game/Blueprints/Nexus_GameInstance.Nexus_GameInstance_C|GetKeystone_1 _asnexus_game_instance))
  (Default|AddKeystone _asthird_person_character)
  (Audio|PlaySoundatLocation "/Game/Blueprints/BlueprintStuff/KeystonePickupWidget/UMG/Keystone-Activation.Keystone-Activation" (Transformation|GetActorLocation))
  (Actor|DestroyActor)
  (Effects|SpawnEmitteratLocation "/Game/StarterContent/Particles/P_Explosion.P_Explosion" (Transformation|GetActorLocation))
  (Variables|/Game/Blueprints/Nexus_GameInstance.Nexus_GameInstance_C|SetCollected_1 _asnexus_game_instance true))

(event EventBeginPlay
  (bind _asnexus_game_instance (Utilities|Casting|CastToNexus_GameInstance (Game|GetGameInstance)))
  (if (Variables|/Game/Blueprints/Nexus_GameInstance.Nexus_GameInstance_C|GetCollected_1 _asnexus_game_instance)
    (Actor|DestroyActor)))

(fn ConstructionScript)