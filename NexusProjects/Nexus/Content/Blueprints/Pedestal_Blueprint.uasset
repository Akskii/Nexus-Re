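; Pedestal that displays the four keystones the player has collected and triggers the end-game state once all are present.
; On box overlap, it checks the Nexus_GameInstance inventory, reveals each held keystone with a sound and sets its Bridge flag; Added guards are never set here.
; Holding all four sets EndGame and runs a timeline driving emissive intensity through a material parameter collection.
; BeginPlay restores keystones and glow from saved Bridge flags.
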(event OnComponentBeginOverlap(Box)
  (params (OtherActor :type Actor%20Object%20Reference) (OtherComp :type Primitive%20Component%20Object%20Reference) (OtherBodyIndex :type Integer) (bFromSweep :type Boolean) (SweepResult :type Hit%20Result%20Structure%20%28by%20ref%29))
  (bind _asnexus_game_instance (Utilities|Casting|CastToNexus_GameInstance (Game|GetGameInstance)))
  (if (not (Variables|/Game/Blueprints/Nexus_GameInstance.Nexus_GameInstance_C|GetEnd%20Game _asnexus_game_instance))
    (if (Utilities|Array|ContainsItem (Variables|/Game/Blueprints/Nexus_GameInstance.Nexus_GameInstance_C|GetInventory _asnexus_game_instance) (Variables|/Game/Blueprints/Nexus_GameInstance.Nexus_GameInstance_C|GetKeystone_1 _asnexus_game_instance))
      (if (Variables|Default|GetAdded_1)
        _
        (else
          (Rendering|SetVisibility (Variables|Default|GetKeystone_1) true false)
          (Audio|PlaySound2D "/Game/Blueprints/BlueprintStuff/KeystonePickupWidget/UMG/Keystone-Activation.Keystone-Activation")
          (Variables|/Game/Blueprints/Nexus_GameInstance.Nexus_GameInstance_C|SetBridge_1 _asnexus_game_instance true))))
    (if (Utilities|Array|ContainsItem (Variables|/Game/Blueprints/Nexus_GameInstance.Nexus_GameInstance_C|GetInventory _asnexus_game_instance) (Variables|/Game/Blueprints/Nexus_GameInstance.Nexus_GameInstance_C|GetKeystone_2 _asnexus_game_instance))
      (if (Variables|Default|GetAdded_2)
        _
        (else
          (Rendering|SetVisibility (Variables|Default|GetKeystone_2) true false)
          (Audio|PlaySound2D "/Game/Blueprints/BlueprintStuff/KeystonePickupWidget/UMG/Keystone-Activation.Keystone-Activation")
          (Variables|/Game/Blueprints/Nexus_GameInstance.Nexus_GameInstance_C|SetBridge_2 _asnexus_game_instance true))))
    (if (Utilities|Array|ContainsItem (Variables|/Game/Blueprints/Nexus_GameInstance.Nexus_GameInstance_C|GetInventory _asnexus_game_instance) (Variables|/Game/Blueprints/Nexus_GameInstance.Nexus_GameInstance_C|GetKeystone_3 _asnexus_game_instance))
      (if (Variables|Default|GetAdded_3)
        _
        (else
          (Rendering|SetVisibility (Variables|Default|GetKeystone_3) true false)
          (Audio|PlaySound2D "/Game/Blueprints/BlueprintStuff/KeystonePickupWidget/UMG/Keystone-Activation.Keystone-Activation")
          (Variables|/Game/Blueprints/Nexus_GameInstance.Nexus_GameInstance_C|SetBridge_3 _asnexus_game_instance true))))
    (if (Utilities|Array|ContainsItem (Variables|/Game/Blueprints/Nexus_GameInstance.Nexus_GameInstance_C|GetInventory _asnexus_game_instance) (Variables|/Game/Blueprints/Nexus_GameInstance.Nexus_GameInstance_C|GetKeystone_4 _asnexus_game_instance))
      (if (Variables|Default|GetAdded_4)
        _
        (else
          (Audio|PlaySound2D "/Game/Blueprints/BlueprintStuff/KeystonePickupWidget/UMG/Keystone-Activation.Keystone-Activation")
          (Rendering|SetVisibility (Variables|Default|GetKeystone_4) true false)
          (Variables|/Game/Blueprints/Nexus_GameInstance.Nexus_GameInstance_C|SetBridge_4 _asnexus_game_instance true))))
    (if (Math|Boolean|ANDBoolean (Utilities|Array|ContainsItem (Variables|/Game/Blueprints/Nexus_GameInstance.Nexus_GameInstance_C|GetInventory _asnexus_game_instance) (Variables|/Game/Blueprints/Nexus_GameInstance.Nexus_GameInstance_C|GetKeystone_1 _asnexus_game_instance)) (Utilities|Array|ContainsItem (Variables|/Game/Blueprints/Nexus_GameInstance.Nexus_GameInstance_C|GetInventory _asnexus_game_instance) (Variables|/Game/Blueprints/Nexus_GameInstance.Nexus_GameInstance_C|GetKeystone_2 _asnexus_game_instance)) (Utilities|Array|ContainsItem (Variables|/Game/Blueprints/Nexus_GameInstance.Nexus_GameInstance_C|GetInventory _asnexus_game_instance) (Variables|/Game/Blueprints/Nexus_GameInstance.Nexus_GameInstance_C|GetKeystone_3 _asnexus_game_instance)) (Utilities|Array|ContainsItem (Variables|/Game/Blueprints/Nexus_GameInstance.Nexus_GameInstance_C|GetInventory _asnexus_game_instance) (Variables|/Game/Blueprints/Nexus_GameInstance.Nexus_GameInstance_C|GetKeystone_4 _asnexus_game_instance)))
      (bind _asnexus_game_instance_2 (Utilities|Casting|CastToNexus_GameInstance (Game|GetGameInstance)))
      (Variables|/Game/Blueprints/Nexus_GameInstance.Nexus_GameInstance_C|SetEnd%20Game _asnexus_game_instance_2 true)
      (bind _newtrack_0 (Timeline|Timeline_0 PlayFromStart)
        (:Update
          (Rendering|Material|SetScalarParameterValue "/Game/Materials/Textures/Pedestal_Parameters.Pedestal_Parameters" "EmissiveIntensity" _newtrack_0 :!class /Script/Engine.KismetMaterialLibrary))))))

(event EventBeginPlay
  (bind _asnexus_game_instance (Utilities|Casting|CastToNexus_GameInstance (Game|GetGameInstance)))
  (if (Variables|/Game/Blueprints/Nexus_GameInstance.Nexus_GameInstance_C|GetBridge_1 _asnexus_game_instance)
    (Rendering|SetVisibility (Variables|Default|GetKeystone_1) true false))
  (if (Variables|/Game/Blueprints/Nexus_GameInstance.Nexus_GameInstance_C|GetBridge_2 _asnexus_game_instance)
    (Rendering|SetVisibility (Variables|Default|GetKeystone_2) true false))
  (if (Variables|/Game/Blueprints/Nexus_GameInstance.Nexus_GameInstance_C|GetBridge_3 _asnexus_game_instance)
    (Rendering|SetVisibility (Variables|Default|GetKeystone_3) true false))
  (if (Variables|/Game/Blueprints/Nexus_GameInstance.Nexus_GameInstance_C|GetBridge_4 _asnexus_game_instance)
    (Rendering|SetVisibility (Variables|Default|GetKeystone_4) true false))
  (if (Math|Boolean|ANDBoolean (Variables|/Game/Blueprints/Nexus_GameInstance.Nexus_GameInstance_C|GetBridge_1 _asnexus_game_instance) (Variables|/Game/Blueprints/Nexus_GameInstance.Nexus_GameInstance_C|GetBridge_2 _asnexus_game_instance) (Variables|/Game/Blueprints/Nexus_GameInstance.Nexus_GameInstance_C|GetBridge_3 _asnexus_game_instance) (Variables|/Game/Blueprints/Nexus_GameInstance.Nexus_GameInstance_C|GetBridge_4 _asnexus_game_instance))
    (Rendering|Material|SetScalarParameterValue "/Game/Materials/Textures/Pedestal_Parameters.Pedestal_Parameters" "EmissiveIntensity" 2e+01 :!class /Script/Engine.KismetMaterialLibrary)))

(fn ConstructionScript)