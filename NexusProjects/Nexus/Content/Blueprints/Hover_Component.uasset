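; Scene component that hovers a physics-simulated bike mesh, handed to it through InitComponent, above surfaces below it.
; Each tick it traces down its local axis and pushes the mesh along the hit normal at its own location, weakening with distance.
; On a hit, linear and angular damping act as throttle and brakes, driven by polled keys, forward speed and the game instance's OffBike flag.
; Without a hit, damping drops for airborne movement.
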(event Custom|InitComponent
  (params (MeshComponent :type Static%20Mesh%20Component%20Object%20Reference))
  ;[1 1 1] Simulate Physics
  (bind _output_get (Variables|Default|SetParentComponent MeshComponent))
  (Physics|SetSimulatePhysics _output_get true))

(event EventTick
  (params (DeltaSeconds :type Float%20%28single-precision%29))
  (bind _returnvalue (Transformation|GetWorldLocation))
  (bind _returnvalue_2 (Game|GetPlayerController 0))
  (bind _parentcomponent (Variables|Default|GetParentComponent))
  (bind _parentcomponent_2 (Variables|Default|GetParentComponent))
  (bind _parentcomponent_3 (Variables|Default|GetParentComponent))
  (bind _returnvalue_3 (Class|PlayerController|GetInputKeyTimeDown _returnvalue_2 "Gamepad_LeftTrigger"))
  (bind _returnvalue_4 (Game|Player|IsInputKeyDown _returnvalue_2 "SpaceBar"))
  (bind _returnvalue_5 (Game|Player|IsInputKeyDown _returnvalue_2 "W"))
  (bind _returnvalue_6 (Class|PlayerController|GetInputKeyTimeDown _returnvalue_2 "SpaceBar"))
  (bind _returnvalue_7 (Math|Float|SelectFloat _returnvalue_6 _returnvalue_3 _returnvalue_4))
  (bind _returnvalue_8 (* _returnvalue_7 12.0))
  (bind _returnvalue_9 (Math|Float|Clamp(Float) _returnvalue_8 1.0 56.98))
  ;[1 1 1] Create Line Trace
  (bind (_outhit _returnvalue_10) (Collision|LineTraceByChannel _returnvalue (+ _returnvalue (* (Math|Vector|GetUpVector) (* (Variables|Default|GetTraceLength) -1.0))) "TraceTypeQuery1" false 0 "None"))
  ;[1 1 1] Did Line Trace hit?
  (if _returnvalue_10
    ;[1 1 1] If yes, add hover force...
    (Class|PrimitiveComponent|AddForceatLocation _parentcomponent_2 (* (.ImpactNormal (Collision|BreakHitResult _outhit)) (Math|Float|Lerp (Variables|Default|GetHoverForce) 0.0 (/ (Math|Vector|VectorLength (- (.Location (Collision|BreakHitResult _outhit)) (Transformation|GetWorldLocation))) (Variables|Default|GetTraceLength)))) (Transformation|GetWorldLocation) "None")
    (bind _returnvalue_11 (Physics|GetPhysicsLinearVelocity _parentcomponent_2 "None"))
    ;;[1 1 1] Is W key pressed? If yes, accelerate. If no, Decelerate
    (bind _result (Math|Float|IncrementFloat DeltaSeconds)
      (:%20%20
        (bind _asnexus_game_instance (Utilities|Casting|CastToNexus_GameInstance (Game|GetGameInstance)))
        ;;[1 1 1] Set Damping Values and enable input
        (Class|PrimitiveComponent|SetLinearDamping _parentcomponent_3 (Math|Float|SelectFloat (Math|Float|SelectFloat (* (/ 0.702 (Math|Float|SelectFloat (Math|Float|Clamp(Float) (* (Math|Float|SelectFloat (Class|PlayerController|GetInputKeyTimeDown _returnvalue_2 "W") (Class|PlayerController|GetInputKeyTimeDown _returnvalue_2 "Gamepad_RightTrigger") _returnvalue_5) 0.5) 0.1 0.54) (Math|Float|Clamp(Float) (/ 1.0 _result) 0.1 1.0) (or _returnvalue_5 (Game|Player|IsInputKeyDown _returnvalue_2 "Gamepad_RightTrigger")))) _returnvalue_9) 5e+01 (or (or (Game|Player|IsInputKeyDown _returnvalue_2 "W") (Game|Player|IsInputKeyDown _returnvalue_2 "Gamepad_RightTrigger")) (> (Math|Float|Absolute(Float) (Math|Vector|DotProduct _returnvalue_11 (Math|Vector|GetForwardVector _parentcomponent_2))) 8.0))) 4e+01 (not (Variables|/Game/Blueprints/Nexus_GameInstance.Nexus_GameInstance_C|GetOff%20Bike? _asnexus_game_instance))))
        (Class|PrimitiveComponent|SetAngularDamping _parentcomponent_3 (Math|Float|SelectFloat (Math|Float|SelectFloat (* (Math|Float|Clamp(Float) _returnvalue_9 1.0 4e+01) 6.0) 5e+01 (or (or (Game|Player|IsInputKeyDown _returnvalue_2 "W") (Game|Player|IsInputKeyDown _returnvalue_2 "Gamepad_RightTrigger")) (> (Math|Float|Absolute(Float) (Math|Vector|DotProduct _returnvalue_11 (Math|Vector|GetForwardVector _parentcomponent_2))) 8.0))) 4e+01 (not (Variables|/Game/Blueprints/Nexus_GameInstance.Nexus_GameInstance_C|GetOff%20Bike? _asnexus_game_instance))))))
    (else
      ;[1 1 1] If no, lower damping values and Disable input
      (Class|PrimitiveComponent|AddForceatLocation _parentcomponent (* (.ImpactNormal (Collision|BreakHitResult _outhit)) (Math|Float|Lerp (Variables|Default|GetHoverForce) 0.0 (/ (Math|Vector|VectorLength (- (.Location (Collision|BreakHitResult _outhit)) (Transformation|GetWorldLocation))) (Variables|Default|GetTraceLength)))) (Transformation|GetWorldLocation) "None")
      (Class|PrimitiveComponent|SetLinearDamping _parentcomponent 0.0)
      (Class|PrimitiveComponent|SetAngularDamping _parentcomponent 8.0))))