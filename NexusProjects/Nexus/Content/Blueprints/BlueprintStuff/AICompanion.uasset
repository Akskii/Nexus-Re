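; AI companion that hovers after the player on foot or the player's bike, taking both from Nexus_GameInstance.
; Until GameStart it stays dark and frozen, then timelines fade in lights and emissive, ease damping and enable physics.
; Tick accelerates the physics capsule toward an offset point, with looser tuning on foot, tilting the mesh by velocity.
; A random timed toggle switches between facing the target and matching its rotation, driving a material parameter.
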(event EventTick
  (params (DeltaSeconds :type Float%20%28single-precision%29))
  (bind _returnvalue (Game|GetPlayerCharacter 0))
  (bind _capsulecomponent (Variables|Collision|GetCapsuleComponent))
  (bind _capsulecomponent_2 (Variables|Collision|GetCapsuleComponent))
  (Rendering|Material|SetScalarParameterValue "/Game/Materials/Textures/Companion_FacePlate/Companion.Companion" "Alpha" (Math|Conversions|ToFloat(Boolean) (Variables|Default|GetLook%20At%20charcter)) :!class /Script/Engine.KismetMaterialLibrary)
  (bind _asnexus_game_instance (Utilities|Casting|CastToNexus_GameInstance (Game|GetGameInstance)))
  (Variables|Default|SetOn%20foot? (Variables|/Game/Blueprints/Nexus_GameInstance.Nexus_GameInstance_C|GetOff%20Bike? _asnexus_game_instance))
  (if (not (Variables|/Game/Blueprints/Nexus_GameInstance.Nexus_GameInstance_C|GetOff%20Bike? _asnexus_game_instance))
    (Variables|Default|SetPreferred%20Rotation (Math|Rotator|SelectRotator (Math|Rotator|FindLookatRotation (Transformation|GetActorLocation) (.Location (Math|Transform|BreakTransform (Variables|/Game/Blueprints/Nexus_GameInstance.Nexus_GameInstance_C|GetBikeTransform _asnexus_game_instance)))) (.Rotation (Math|Transform|BreakTransform (Variables|/Game/Blueprints/Nexus_GameInstance.Nexus_GameInstance_C|GetBikeTransform _asnexus_game_instance))) (Variables|Default|GetLook%20At%20charcter)))
    (Variables|Default|SetPreferred%20Location (+ (.Location (Math|Transform|BreakTransform (Variables|/Game/Blueprints/Nexus_GameInstance.Nexus_GameInstance_C|GetBikeTransform _asnexus_game_instance))) "100.000000,100.000000,160.000000"))
    (Variables|Default|SetMax%20Acceleration 9.9e+04)
    (Variables|Default|SetRotateMaxSpeed 1.8e+03)
    (Class|PrimitiveComponent|SetLinearDamping (Variables|Collision|GetCapsuleComponent) 17.0)
    (else
      (Variables|Default|SetPreferred%20Rotation (Math|Rotator|SelectRotator (Math|Rotator|FindLookatRotation (Transformation|GetActorLocation) (Transformation|GetActorLocation (Game|GetPlayerCharacter 0))) (Transformation|GetActorRotation _returnvalue) (Variables|Default|GetLook%20At%20charcter)))
      (Variables|Default|SetPreferred%20Location (+ (Transformation|GetActorLocation _returnvalue) "110.000000,110.000000,20.000000"))
      (Variables|Default|SetMax%20Acceleration 8e+02)
      (Variables|Default|SetRotateMaxSpeed 8e+02)
      (Class|PrimitiveComponent|SetLinearDamping (Variables|Collision|GetCapsuleComponent) 1.7)))
  ;[1 1 1] Rotation
  (Variables|Default|SetRotateSpeed (Math|Float|SelectFloat (+ (* (Variables|Default|GetRotateAccel) DeltaSeconds) (Variables|Default|GetRotateSpeed)) (* (Variables|Default|GetRotateMaxSpeed) (- 1.0 (Math|Vector|DotProduct (Math|Vector|GetForwardVector (Transformation|GetActorRotation)) (Math|Vector|GetForwardVector (Variables|Default|GetPreferred%20Rotation))))) (< (Variables|Default|GetRotateSpeed) (* (Variables|Default|GetRotateMaxSpeed) (- 1.0 (Math|Vector|DotProduct (Math|Vector|GetForwardVector (Transformation|GetActorRotation)) (Math|Vector|GetForwardVector (Variables|Default|GetPreferred%20Rotation))))))))
  (bind _asnexus_game_instance_2 (Utilities|Casting|CastToNexus_GameInstance (Game|GetGameInstance)))
  (if (Variables|/Game/Blueprints/Nexus_GameInstance.Nexus_GameInstance_C|GetGameStart? _asnexus_game_instance_2)
    (if (Variables|Default|GetJust%20Delayed?) :!label _label
      (Audio|Components|Audio|Play (Variables|Character|GetMesh) true)
      (Collision|SetCollisionEnabled (Variables|Collision|GetCapsuleComponent) "PhysicsOnly")
      (bind _returnvalue_2 (Physics|GetPhysicsLinearVelocity _capsulecomponent "None"))
      (if (> (Math|Vector|DotProduct _returnvalue_2 (Math|Vector|GetForwardVector _capsulecomponent)) 0.0)
        (Transformation|SetRelativeRotation (Variables|Character|GetMesh) (Math|Rotator|MakeRotator (Math|Float|Clamp(Float) (* (Math|Float|Absolute(Float) (.X (Math|Vector|BreakVector _returnvalue_2))) -0.041) -45.0 0.0) (Math|Float|Clamp(Float) (* (Math|Float|Absolute(Float) (.Y (Math|Vector|BreakVector _returnvalue_2))) -0.041) -45.0 0.0) 0.0) false false)
        (else
          (Transformation|SetRelativeRotation (Variables|Character|GetMesh) (Math|Rotator|MakeRotator (Math|Float|Clamp(Float) (* (Math|Float|Absolute(Float) (.X (Math|Vector|BreakVector _returnvalue_2))) 0.041) 0.0 45.0) (Math|Float|Clamp(Float) (* (Math|Float|Absolute(Float) (.Y (Math|Vector|BreakVector _returnvalue_2))) 0.041) 0.0 45.0) 0.0) false false)))
      (Transformation|SetWorldRotation _capsulecomponent_2 (Class|KismetMathLibrary|RInterptoConstant (Transformation|GetActorRotation) (Variables|Default|GetPreferred%20Rotation) DeltaSeconds (Variables|Default|GetRotateSpeed)) false false)
      ;[1 1 1] Movement
      (Physics|SetPhysicsLinearVelocity _capsulecomponent_2 (* (Math|Vector|SelectVector (* (Math|Vector|Normalize (* (- (Variables|Default|GetPreferred%20Location) (Transformation|GetActorLocation)) (Variables|Default|GetAcceleration))) (Variables|Default|GetMax%20Acceleration)) (* (- (Variables|Default|GetPreferred%20Location) (Transformation|GetActorLocation)) (Variables|Default|GetAcceleration)) (> (Math|Vector|VectorLength (* (- (Variables|Default|GetPreferred%20Location) (Transformation|GetActorLocation)) (Variables|Default|GetAcceleration))) (Variables|Default|GetMax%20Acceleration))) DeltaSeconds) true "None")
      (else
        (Utilities|FlowControl|Delay 3.0)
        (Variables|Default|SetJust%20Delayed? true)
        (goto _label)))))

(event EventBeginPlay
  (bind _companionhover (Variables|Default|GetCompanionHover))
  (bind _asnexus_game_instance (Utilities|Casting|CastToNexus_GameInstance (Game|GetGameInstance)))
  (if (Variables|/Game/Blueprints/Nexus_GameInstance.Nexus_GameInstance_C|GetGameStart? _asnexus_game_instance) :!label _label
    (bind _newtrack_8 (Timeline|Timeline_0 PlayFromStart)
      (:Update
        (Rendering|Components|Light|SetIntensity (Variables|Default|GetFaceLight) (* _newtrack_8 5.0))
        (Rendering|Components|Light|SetIntensity (Variables|Default|GetCompanionEmitterLight) (* _newtrack_8 1.2e+02))
        (Rendering|Material|SetScalarParameterValue "/Game/Materials/Textures/Companion_FacePlate/Companion.Companion" "EmissiveIntensity" (* _newtrack_8 2.0) :!class /Script/Engine.KismetMaterialLibrary)
        (Components|Activation|SetActive (Variables|Default|GetCompanionWings_L) true false)
        (Utilities|FlowControl|Delay 2.0)
        (bind (_direction _newtrack_0 _newtrack_1) (Timeline|Timeline_1 PlayFromStart)
          (:Update
            (Class|PrimitiveComponent|SetLinearDamping (Variables|Collision|GetCapsuleComponent) _newtrack_0)
            (Class|PrimitiveComponent|SetAngularDamping (Variables|Collision|GetCapsuleComponent) _newtrack_1)
            (Utilities|FlowControl|Delay 0.5)
            (Physics|SetSimulatePhysics (Variables|Collision|GetCapsuleComponent) true)
            (Collision|SetCollisionEnabled (Variables|Collision|GetCapsuleComponent) "PhysicsOnly")
            (Components|Activation|Activate _companionhover false)
            (Audio|Components|Audio|Play _companionhover 0.0)
            (bind _output_get (Variables|Default|SetLook%20At%20charcter (Math|Random|RandomBool) :!label _label_2))
            (if _output_get
              (Utilities|FlowControl|Delay 2.0)
              (goto _label_2)
              (else
                (Utilities|FlowControl|Delay 7.0)
                (goto _label_2)))))))
    (else
      (Components|Activation|SetActive (Variables|Default|GetCompanionWings_L) false false)
      (Rendering|Components|Light|SetIntensity (Variables|Default|GetFaceLight) 0.0)
      (Audio|Components|Audio|Stop (Variables|Character|GetMesh))
      (Physics|SetSimulatePhysics (Variables|Collision|GetCapsuleComponent) false)
      (Collision|SetCollisionEnabled (Variables|Collision|GetCapsuleComponent) "NoCollision")
      (Class|PrimitiveComponent|SetLinearDamping (Variables|Collision|GetCapsuleComponent) 5e+02)
      (Class|PrimitiveComponent|SetAngularDamping (Variables|Collision|GetCapsuleComponent) 5e+02)
      (Utilities|FlowControl|Delay 1.0)
      (goto _label))))

(fn ConstructionScript)