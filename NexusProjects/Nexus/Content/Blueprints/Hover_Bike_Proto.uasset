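; Prototype physics-driven hover bike that responds to player input for driving and camera aim.
; Four hover components are initialized with the bike mesh on BeginPlay, while input axes apply forward/backward force and yaw torque to that mesh.
; Steering torque flips when the bike is not moving forward, using a velocity-to-forward dot product.
; Turn input yaws the spring arm independently, and a radial force node is left unconnected.
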(event EventBeginPlay
  (bind _bikemesh (Variables|Default|GetBikeMesh))
  ;[1 1 1] Hover Components
  (Default|InitComponent (Variables|Default|GetHover_Component1) _bikemesh)
  (Default|InitComponent (Variables|Default|GetHover_Component2) _bikemesh)
  (Default|InitComponent (Variables|Default|GetHover_Component3) _bikemesh)
  (Default|InitComponent (Variables|Default|GetHover_Component4) _bikemesh))

(event Input|AxisEvents|InputAxisMoveForward
  (params (AxisValue :type Float%20%28single-precision%29))
  ;[1 1 1] Forwards/Backwards Movement
  (Physics|AddForce (Variables|Default|GetBikeMesh) (* (* (Math|Vector|GetForwardVector (Variables|Default|GetBikeMesh)) 8e+05) AxisValue) "None" false))

(event Input|AxisEvents|InputAxisTurn
  (params (AxisValue :type Float%20%28single-precision%29))
  ;[1 1 1] Camera Aim
  (Transformation|AddRelativeRotation (Variables|Default|GetSpringArm) (Math|Rotator|MakeRotator 0.0 0.0 (* AxisValue 1.0)) false false))

(event Input|AxisEvents|InputAxisMoveRight
  (params (AxisValue :type Float%20%28single-precision%29))
  ;[1 1 1] Vehicle Turning
  (bind _returnvalue (Physics|GetPhysicsLinearVelocity (Variables|Default|GetBikeMesh) "None"))
  (Class|PrimitiveComponent|AddTorque (Variables|Default|GetBikeMesh) (Math|Vector|MakeVector 0.0 0.0 (* (Math|Float|SelectFloat 1.0 -1.0 (> (Math|Vector|DotProduct _returnvalue (Math|Vector|GetForwardVector (Variables|Default|GetBikeMesh))) 0.0)) (* AxisValue 1.4e+06))) "None" false))

(fn ConstructionScript)